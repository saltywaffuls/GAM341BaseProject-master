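; B_Boss is a boss AI whose capsule hit sends the player back to the last checkpoint.
; On any hit, without checking the other actor, it disables player input and waits briefly.
; If the "check" save slot exists, it loads the B_savepoint save, moves the player to the stored location and restores input.
; Otherwise it opens a level by name to restart.
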(event `self.CapsuleComponent.OnComponentHit`
  (params (HitComponent :type "PrimitiveComponent Object Reference") (OtherActor :type "Actor Object Reference") (OtherComp :type "PrimitiveComponent Object Reference") (NormalImpulse :type "Vector Structure") (Hit :type "HitResult Structure (by ref)"))
  (`KismetSystemLibrary.PrintString` "ai hit")
  (bind _assimple_character (cast `/Game/Blueprints/BasicPlayer/simple_Character` (`GameplayStatics.GetPlayerCharacter` 0)))
  (`self.DisableInput` _assimple_character (`GameplayStatics.GetPlayerController` 0))
  (`KismetSystemLibrary.Delay` 2.0)
  (bind _returnvalue (`GameplayStatics.DoesSaveGameExist` "check"))
  (if _returnvalue
    (bind _returnvalue_2 (`GameplayStatics.LoadGameFromSlot` "check"))
    (bind _asb_savepoint (cast `/Game/Blueprints/B_savepoint` _returnvalue_2))
    (bind _assimple_character_2 (cast `/Game/Blueprints/BasicPlayer/simple_Character` (`GameplayStatics.GetPlayerCharacter` 0)))
    (`self.K2_SetActorLocation` _assimple_character_2 (`/Game/Blueprints/B_savepoint.Player_location` _asb_savepoint) false false)
    (`self.EnableInput` _assimple_character_2 (`GameplayStatics.GetPlayerController` 0))
    (else
      (`GameplayStatics.OpenLevel` (`self.level`)))))

(fn `UserConstructionScript`)