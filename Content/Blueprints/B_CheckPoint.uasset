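; Checkpoint trigger actor that either records or clears the player's saved checkpoint when its Trigger component is overlapped, depending on its Load flag.
; With Load set, it writes the simple_Character's location and a true Load flag to a B_savepoint in slot "check", creating the save if none exists.
; Otherwise it sets the existing save's Load flag to false, keeping the stored location.
; The overlap does not filter which actor entered.
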(event `self.trigger.OnComponentBeginOverlap`
  (params (OverlappedComponent :type "PrimitiveComponent Object Reference") (OtherActor :type "Actor Object Reference") (OtherComp :type "PrimitiveComponent Object Reference") (OtherBodyIndex :type Integer) (bFromSweep :type Boolean) (SweepResult :type "HitResult Structure (by ref)"))
  (bind _player_location (`self.Player location`))
  (if (`self.Load`)
    (`|ExecutionSequence`
      (:`then_0`
        (bind _assimple_character (cast `/Game/Blueprints/BasicPlayer/simple_Character` (`GameplayStatics.GetPlayerCharacter` 0)))
        (set `self.Player location` (`self.K2_GetActorLocation` _assimple_character)))
      (:`then_1`
        (bind _returnvalue (`GameplayStatics.DoesSaveGameExist` "check"))
        (if _returnvalue
          (bind _returnvalue_2 (`GameplayStatics.LoadGameFromSlot` "check"))
          (bind _asb_savepoint (cast `/Game/Blueprints/B_savepoint` _returnvalue_2))
          (set `/Game/Blueprints/B_savepoint.Player_location` _player_location _asb_savepoint)
          (set `/Game/Blueprints/B_savepoint.load` true _asb_savepoint)
          (`GameplayStatics.SaveGameToSlot` _asb_savepoint "check")
          (`KismetSystemLibrary.PrintString` "checkPoint")
          (else
            (bind _returnvalue_3 (`GameplayStatics.CreateSaveGameObject` "/Game/Blueprints/B_savepoint.B_savepoint_C"))
            (set `/Game/Blueprints/B_savepoint.Player_location` _player_location _returnvalue_3)
            (set `/Game/Blueprints/B_savepoint.load` true _returnvalue_3)
            (`GameplayStatics.SaveGameToSlot` _returnvalue_3 "check")
            (`KismetSystemLibrary.PrintString` "checkPoint")))))
    (else
      (bind _returnvalue_4 (`GameplayStatics.LoadGameFromSlot` "check"))
      (bind _asb_savepoint_2 (cast `/Game/Blueprints/B_savepoint` _returnvalue_4))
      (set `/Game/Blueprints/B_savepoint.load` false _asb_savepoint_2)
      (`GameplayStatics.SaveGameToSlot` _asb_savepoint_2 "check")
      (`KismetSystemLibrary.PrintString` "checkpointClear"))))

(fn `UserConstructionScript`)